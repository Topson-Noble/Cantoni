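; Flying monster that spits bubbles at the hero and also controls the length of the play session.
; A Quartz beat subscription on the audio manager's clock starts a timeline-driven four-corner path loop and a timer spawning bubbles with randomized wobble and speed.
; Tick stops spawning and flags game over on the score manager at a fixed elapsed time.
; The game duration timer saves the score to the leaderboard and opens the score level.
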(event `Gameplay Duration`
  ; Stop spawning bubbles after x seconds
  (set `self.Is Spawning?` false)
  (`KismetSystemLibrary.K2_ClearAndInvalidateTimerHandle` (`self.Game Duration Timer HDL`))
  (`KismetSystemLibrary.K2_ClearAndInvalidateTimerHandle` (`self.Timer HDL`))
  ; Update score
  (bind _save_game_data (message `/Game/Blueprints/Pawn/Save/BPI_SaveGame.GetGameData` (`GameplayStatics.GetGameInstance`)))
  (`/Engine/EditorBlueprintResources/StandardMacros.IsValid` _save_game_data
    (:`Is Valid`
      (bind _player_score (`/Game/Blueprints/Pawn/Save/BP_SaveGame.Player Score` _save_game_data))
      (message `/Game/Blueprints/Pawn/Save/BPI_SaveGame.Save Player Score` (`GameplayStatics.GetGameInstance`) _player_score true)
      ; Add score to Leaderboard
      (message `/Game/Blueprints/Pawn/Save/BPI_SaveGame.Save Score To Leaderboard` (`GameplayStatics.GetGameInstance`) (`/Game/Blueprints/Pawn/Save/BP_SaveGame.Player Name` _save_game_data) _player_score true)
      ; Open leaderboard
      (`KismetSystemLibrary.Delay` 0.5)
      (`GameplayStatics.OpenLevelBySoftObjectPtr` "/Game/Levels/PlayerScoreLevel.PlayerScoreLevel"))))

(event `self.ReceiveBeginPlay`
  (`|ExecutionSequence`
    (:`then_0`
      ; Reference hero
      (bind _returnvalue (`GameplayStatics.GetActorOfClass` "/Game/Blueprints/Characters/Hero/BP_Hero.BP_Hero_C"))
      (set `self.Target Actor` _returnvalue)
      ; Stop spawning bubbles after x seconds
      (bind _returnvalue_2 (`KismetSystemLibrary.K2_SetTimerDelegate` (delegate `Gameplay Duration`) (`self.Game Duration`)))
      (set `self.Game Duration Timer HDL` _returnvalue_2))
    (:`then_1`
      ; Initial setups
      (`CharacterMovementComponent.SetMovementMode` (`self.CharacterMovement`) "MOVE_Flying" 0)
      (bind _returnvalue_3 (`GameplayStatics.GetActorOfClass` "/Game/Blueprints/Pawn/BP_AudioManager.BP_AudioManager_C"))
      (set `self.Audio Manager REF` _returnvalue_3)
      (`self.K2_SetActorLocation` (0.0 300.0 140.0))
      (`QuartzClockHandle.SubscribeToQuantizationEvent` (`/Game/Blueprints/Pawn/BP_AudioManager.Clock HDL` (`self.Audio Manager REF`)) "Beat" (delegate `Start Moving Character`)))
    (:`then_2`
      ; Reference score manager
      (bind _returnvalue_4 (`GameplayStatics.GetActorOfClass` "/Game/Blueprints/Pawn/BP_ScoreManager.BP_ScoreManager_C"))
      (set `self.Score Manager REF` _returnvalue_4))))

(event `Start Moving Character`
  (params (ClockName :type Name) (QuantizationType :type "EQuartzCommandQuantization Enum" :default "Bar") (NumBars :type Integer) (Beat :type Integer) (BeatFraction :type "Float (single-precision)"))
  ; Start movement
  (if (== NumBars 3)
    (`/Engine/EditorBlueprintResources/StandardMacros.DoOnce` false
      (:`Completed`
        (set `self.Path Index` 0)
        (`self.Start Path Loop`)
        (`SkeletalMeshComponent.PlayAnimation` (`self.Mesh`) "/Game/Assets/Characters/MonsterCharacter/Animation/Monster_Anim.Monster_Anim" true)
        ; Spawn bubbles every x seconds
        (bind _returnvalue (`KismetSystemLibrary.K2_SetTimerDelegate` (delegate `Spawn Bubble`) 0.35 true))
        (set `self.Timer HDL` _returnvalue)))))

(event `Spawn Bubble`
  ; Spawn bubbles every x seconds
  (if (`self.Is Spawning?`)
    (`GameplayStatics.PlaySound2D` "/Game/Assets/Sounds/spit_out_sfx_2_Cue.spit_out_sfx_2_Cue" 1.0 1.0 0.0 null null)
    ; Spawn bubbles from the source, and direct towards target
    (bind _returnvalue (`|SpawnActorFromClass` "/Game/Blueprints/Characters/Bubble/BP_Bubble.BP_Bubble_C" (`KismetMathLibrary.MakeTransform` (`self.K2_GetActorLocation`) (struct) (0.1 1.0 1.0)) "Undefined" "MultiplyWithRoot" null null))
    (`PrimitiveComponent.IgnoreActorWhenMoving` (`self.Mesh`) _returnvalue true)
    (set `/Game/Blueprints/Characters/Bubble/BP_Bubble.Target Location` (`self.K2_GetActorLocation` (`self.Target Actor`)) _returnvalue)
    (set `/Game/Blueprints/Characters/Bubble/BP_Bubble.Wobble Amplitude` (`KismetMathLibrary.RandomFloatInRange` 60.0 120.0) _returnvalue)
    (set `/Game/Blueprints/Characters/Bubble/BP_Bubble.Wobble Frequency` (`KismetMathLibrary.RandomFloatInRange` 2.0 4.0) _returnvalue)
    (set `/Game/Blueprints/Characters/Bubble/BP_Bubble.Movement Speed` (`KismetMathLibrary.RandomFloatInRange` 300.0 320.0) _returnvalue)))

(event `Start Path Loop`
  ; Loop logic
  (set `self.Start Position Vector` (`self.K2_GetActorLocation`))
  (switch `int` (`self.Path Index`)
    (:`0`
      (set `self.End Position Vector` (0.0 -300.0 130.0))
      (bind (_direction _move) (`Timeline|Move Animation` :!via `PlayFromStart` :!label _label)
        (:`Update`
          (`self.K2_SetActorLocation` (`KismetMathLibrary.VLerp` (`self.Start Position Vector`) (`self.End Position Vector`) _move)))
        (:`Finished`
          (set `self.Path Index` (mod (+ (`self.Path Index`) 1) 4))
          (`self.Start Path Loop`))))
    (:`1`
      (set `self.End Position Vector` (0.0 -300.0 -130.0))
      (goto _label :!via `PlayFromStart`))
    (:`2`
      (set `self.End Position Vector` (0.0 300.0 -130.0))
      (goto _label :!via `PlayFromStart`))
    (:`3`
      (set `self.End Position Vector` (0.0 300.0 130.0))
      (goto _label :!via `PlayFromStart`))))

(event `self.ReceiveTick`
  (params (DeltaSeconds :type "Float (single-precision)"))
  ; Stop spawning bubbles after X seconds
  (if (>= (`KismetSystemLibrary.K2_GetTimerElapsedTimeHandle` (`self.Game Duration Timer HDL`)) 80.0)
    (`/Engine/EditorBlueprintResources/StandardMacros.DoOnce` false
      (:`Completed`
        (bind _output_get (set `self.Bubble spawn time min` 0.0))
        (set `self.Bubble spawn time max` _output_get)
        (set `self.Is Spawning?` false)
        (set `/Game/Blueprints/Pawn/BP_ScoreManager.Is Game Over?` true (`self.Score Manager REF`))))))

(fn `UserConstructionScript`)