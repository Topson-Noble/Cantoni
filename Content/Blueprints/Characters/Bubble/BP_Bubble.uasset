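; Bubble actor that drifts toward a target location and is popped by clicking for points, or costs points when it hits a hero.
; Tick moves it toward the target with a sine-driven sideways wobble from a cross product with world up.
; Clicking its sphere increments the score, while overlapping a BPI_CanCollide actor decrements it.
; Both play effects, update BP_ScoreManager's HUD, save asynchronously through the GameInstance, and destroy the bubble.
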(event `self.ReceiveTick`
  (params (DeltaSeconds :type "Float (single-precision)"))
  (bind _returnvalue (`KismetMathLibrary.Normal` (- (`self.Target Location`) (`self.K2_GetActorLocation`))))
  ; Bubble wobbly movements
  (`self.K2_SetActorLocation` (+ (+ (* _returnvalue DeltaSeconds (`self.Movement Speed`)) (* DeltaSeconds (* (`KismetMathLibrary.Cross_VectorVector` _returnvalue (`KismetMathLibrary.MakeVector` 0.0 0.0 1.0)) (* (`KismetMathLibrary.Sin` (* (`KismetSystemLibrary.GetGameTimeInSeconds`) (`self.Wobble Frequency`))) (`self.Wobble Amplitude`))))) (`self.K2_GetActorLocation`))))

(event `self.Trigger volume.OnComponentBeginOverlap`
  (params (OverlappedComponent :type "PrimitiveComponent Object Reference") (OtherActor :type "Actor Object Reference") (OtherComp :type "PrimitiveComponent Object Reference") (OtherBodyIndex :type Integer) (bFromSweep :type Boolean) (SweepResult :type "HitResult Structure (by ref)"))
  ; Destroy self upon interacting with heros
  (if (`KismetSystemLibrary.DoesImplementInterface` OtherActor "/Game/Blueprints/Characters/Hero/BPI_CanCollide.BPI_CanCollide_C")
    (`NiagaraFunctionLibrary.SpawnSystemAtLocation` "/Game/Blueprints/Pawn/BlueBurstFX.BlueBurstFX" (`self.K2_GetActorLocation` OtherActor))
    (`GameplayStatics.PlaySound2D` "/Game/Assets/Sounds/pop_sfx_Cue.pop_sfx_Cue" 1.0 1.0 0.0 null null)
    (bind _returnvalue (`GameplayStatics.GetActorOfClass` "/Game/Blueprints/Pawn/BP_ScoreManager.BP_ScoreManager_C"))
    (bind _result (`/Engine/EditorBlueprintResources/StandardMacros.DecrementInt` (`/Game/Blueprints/Pawn/BP_ScoreManager.Current Score` _returnvalue))
      (:`  `
        (bind _output_get (set `/Game/Blueprints/Pawn/BP_ScoreManager.Current Score` _result _returnvalue))
        (`TextBlock.SetText` (`/Game/Blueprints/Pawn/Widgets/ScoreHUD.SCOREVALUE` (`/Game/Blueprints/Pawn/BP_ScoreManager.Score HUD` _returnvalue)) (`KismetTextLibrary.Conv_IntToText` _output_get))
        (message `/Game/Blueprints/Pawn/Save/BPI_SaveGame.Save Player Score` (`GameplayStatics.GetGameInstance`) _output_get true)
        (`self.K2_DestroyActor`)))))

(event `self.Sphere.OnClicked`
  (params (TouchedComponent :type "PrimitiveComponent Object Reference") (ButtonPressed :type "Key Structure"))
  ; Update score for every bubble bursted
  (`GameplayStatics.PlaySound2D` "/Game/Assets/Sounds/spit_out_sfx_Cue.spit_out_sfx_Cue" 1.0 1.0 0.0 null null)
  (`NiagaraFunctionLibrary.SpawnSystemAtLocation` "/Game/Blueprints/Pawn/PinkBurstFX.PinkBurstFX" (`self.K2_GetActorLocation`))
  (bind _returnvalue (`GameplayStatics.GetActorOfClass` "/Game/Blueprints/Pawn/BP_ScoreManager.BP_ScoreManager_C"))
  (bind _output_get (set `self.Score Manager` _returnvalue))
  (bind _result (`/Engine/EditorBlueprintResources/StandardMacros.IncrementInt` (`/Game/Blueprints/Pawn/BP_ScoreManager.Current Score` _output_get))
    (:`  `
      (bind _output_get_2 (set `/Game/Blueprints/Pawn/BP_ScoreManager.Current Score` _result _output_get))
      (`TextBlock.SetText` (`/Game/Blueprints/Pawn/Widgets/ScoreHUD.SCOREVALUE` (`/Game/Blueprints/Pawn/BP_ScoreManager.Score HUD` _output_get)) (`KismetTextLibrary.Conv_IntToText` _output_get_2))
      ; Save out score
      (message `/Game/Blueprints/Pawn/Save/BPI_SaveGame.Save Player Score` (`GameplayStatics.GetGameInstance`) _output_get_2 true)
      (`self.K2_DestroyActor`))))

(fn `UserConstructionScript`)