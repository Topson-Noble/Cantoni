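; BP_Hero is the hero character Blueprint, which starts a dance animation in sync with the music.
; On BeginPlay it finds BP_AudioManager and subscribes to Bar events on its Quartz clock.
; When the third bar is reported, it plays the looping mesh animation and starts a Timeline that lerps the mesh's relative height for a jump.
; The construction script caches the mesh's world location.
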(event `self.ReceiveBeginPlay`
  ; delay a little before playing dance animation
  (bind _returnvalue (`GameplayStatics.GetActorOfClass` "/Game/Blueprints/Pawn/BP_AudioManager.BP_AudioManager_C"))
  (bind _output_get (set `self.AudioManager REF` _returnvalue))
  (`QuartzClockHandle.SubscribeToQuantizationEvent` (`/Game/Blueprints/Pawn/BP_AudioManager.Clock HDL` _output_get) "Bar" (delegate `Play CharAnim`)))

(event `Play CharAnim`
  (params (ClockName :type Name) (QuantizationType :type "EQuartzCommandQuantization Enum" :default "Bar") (NumBars :type Integer) (Beat :type Integer) (BeatFraction :type "Float (single-precision)"))
  ; delay a little before playing dance animation
  (if (== NumBars 3)
    (`SkeletalMeshComponent.PlayAnimation` (`self.Mesh`) "/Game/Assets/Characters/HeroCharacter/Animation/Char_Anim.Char_Anim" true)
    (`self.Jump Animation`)))

(event `Jump Animation`
  (bind (_direction _jump_up) (`Timeline|Animate Upwards`)
    (:`Update`
      (`SceneComponent.K2_SetRelativeLocation` (`self.Mesh`) (`KismetMathLibrary.MakeVector` 0.0 0.0 (`KismetMathLibrary.Lerp` -40.252333 -25.0 _jump_up)) false false))))

(fn `UserConstructionScript`
  (set `self.Current Location` (`SceneComponent.K2_GetComponentLocation` (`self.Mesh`))))