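; BP_AudioManager starts the game's music on a Quartz clock so that playback is quantized to the bar.
; On BeginPlay it creates the clock, sets its tempo and creates a boosted-volume 2D sound from MSS_Music.
; It queues that sound with PlayQuantized on a bar boundary, and starts the clock only when the Queued event fires, keeping music and clock in step.
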(event `self.ReceiveBeginPlay`
  ; Create new clock
  (bind _returnvalue (`QuartzSubsystem.CreateNewClock` :`self` (subsystem `QuartzSubsystem`) :`ClockName` "Clock01"))
  (bind _clockhandle (`QuartzClockHandle.SetBeatsPerMinute` :`self` _returnvalue :`BeatsPerMinute` 114.0))
  (set `self.Clock HDL` _clockhandle)
  ; Start clock and play audio
  (bind _returnvalue_2 (`GameplayStatics.CreateSound2D` "/Game/Assets/Sounds/MSS_Music.MSS_Music" 1.0 1.0 0.0 null))
  (bind _output_get (set `self.Music REF` _returnvalue_2))
  (`AudioComponent.SetVolumeMultiplier` _returnvalue_2 2.0)
  (`AudioComponent.PlayQuantized` _output_get (`self.Clock HDL`) (make `QuartzQuantizationBoundary` "Bar") (delegate `Start Clock`) 0.0 0.0 1.0 "Linear"))

(event `Start Clock`
  (params (EventType :type "EQuartzCommandDelegateSubType Enum" :default "CommandOnFailedToQueue") (Name :type Name))
  ; Start clock and play audio
  (switch `EQuartzCommandDelegateSubType` EventType
    (:`CommandOnQueued`
      (`QuartzClockHandle.StartClock` (`self.Clock HDL`)))))

(fn `UserConstructionScript`)