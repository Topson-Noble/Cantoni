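; BP_NarrationManager runs an intro narration screen that steps through story lines and then loads the next level.
; On BeginPlay it creates the IntroNarrationHUD widget, shows the mouse cursor, displays the first line and binds the Next button.
; Each click plays a burst effect and pop sound and advances the text.
; When the index reaches the array length, it repeats the burst, waits briefly and opens GameLevel, commented as name input.
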(event `self.ReceiveBeginPlay`
  (bind _returnvalue (`GameplayStatics.GetPlayerController` 0))
  (set `self.Narration Index` 0)
  ; Show narration widget
  (bind _returnvalue_2 (`|CreateWidget` "/Game/Blueprints/Pawn/Widgets/IntroNarrationHUD.IntroNarrationHUD_C"))
  (bind _output_get (set `self.Narration HUD` _returnvalue_2))
  (`UserWidget.AddToViewport` _output_get 0)
  (set `PlayerController.bShowMouseCursor` true _returnvalue)
  (`self.EnableInput` _returnvalue)
  ; Initialize story
  (`TextBlock.SetText` (`/Game/Blueprints/Pawn/Widgets/IntroNarrationHUD.StoryTexts` (`self.Narration HUD`)) (`|GetArrayItem` (`self.Narration Lines`) (`self.Narration Index`)))
  ; Switch story on clicked
  (add `Button.OnClicked` (`/Game/Blueprints/Pawn/Widgets/IntroNarrationHUD.NextButton` (`self.Narration HUD`)) (delegate `OnClicked_Event`)))

(event `OnClicked_Event`
  ; Switch story on clicked
  (`NiagaraFunctionLibrary.SpawnSystemAtLocation` "/Game/Blueprints/Pawn/ButtonPressBurstFX.ButtonPressBurstFX" (0.0 300.0 -140.0))
  (`GameplayStatics.PlaySound2D` "/Game/Assets/Sounds/pop_sfx_Cue.pop_sfx_Cue" 1.0 1.0 0.0 null null)
  (bind _result (`/Engine/EditorBlueprintResources/StandardMacros.IncrementInt` (`self.Narration Index`))
    (:`  `
      (bind _output_get (set `self.Narration Index` _result))
      (`TextBlock.SetText` (`/Game/Blueprints/Pawn/Widgets/IntroNarrationHUD.StoryTexts` (`self.Narration HUD`)) (`|GetArrayItem` (`self.Narration Lines`) _output_get))
      ; Open name input level
      (if (== (`self.Narration Index`) (`KismetArrayLibrary.Array_Length` (`self.Narration Lines`)))
        (`NiagaraFunctionLibrary.SpawnSystemAtLocation` "/Game/Blueprints/Pawn/ButtonPressBurstFX.ButtonPressBurstFX" (0.0 300.0 -140.0))
        (`KismetSystemLibrary.Delay` 1.0)
        (`GameplayStatics.OpenLevelBySoftObjectPtr` "/Game/Levels/GameLevel.GameLevel")))))

(fn `UserConstructionScript`)