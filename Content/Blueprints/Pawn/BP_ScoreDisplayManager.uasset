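; BP_ScoreDisplayManager presents the player's score along with success feedback.
; On BeginPlay it enables input from the first player controller, shows the mouse cursor and adds a PlayerScoreHUD widget to the viewport.
; It plays a success sound and spawns a scaled-down burst effect at the world origin.
; The score text comes from the game data message held by the game instance, set only when that message is valid.
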(event `self.ReceiveBeginPlay`
  (bind _returnvalue (`GameplayStatics.GetPlayerController` 0))
  ; Enable input
  (`self.EnableInput` _returnvalue)
  (set `PlayerController.bShowMouseCursor` true _returnvalue)
  ; Display score widget
  (bind _returnvalue_2 (`|CreateWidget` "/Game/Blueprints/Pawn/Widgets/PlayerScoreHUD.PlayerScoreHUD_C"))
  (bind _output_get (set `self.Player Score HUD` _returnvalue_2))
  (`UserWidget.AddToViewport` _output_get 0)
  (`GameplayStatics.PlaySound2D` "/Game/Assets/Sounds/success_tone_Cue.success_tone_Cue" 1.0 1.0 0.0 null null)
  (`NiagaraFunctionLibrary.SpawnSystemAtLocation` "/Game/Blueprints/Pawn/SuccessBurst.SuccessBurst" (0.0 0.0 0.0) (struct) (0.25 0.25 0.25))
  ; Update player score
  (bind _save_game_data (message `/Game/Blueprints/Pawn/Save/BPI_SaveGame.GetGameData` (`GameplayStatics.GetGameInstance`)))
  (`/Engine/EditorBlueprintResources/StandardMacros.IsValid` _save_game_data
    (:`Is Valid`
      (`TextBlock.SetText` (`/Game/Blueprints/Pawn/Widgets/PlayerScoreHUD.Score` (`self.Player Score HUD`)) (`KismetTextLibrary.Conv_IntToText` (`/Game/Blueprints/Pawn/Save/BP_SaveGame.Player Score` _save_game_data))))))

(fn `UserConstructionScript`)