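; BP_ScoreManager owns the score and pause UI, initializes the score and handles the game-over fadeout.
; BeginPlay enables input, adds the score HUD to the viewport, creates the pause HUD and zeroes the score.
; Tick polls a game-over flag and plays the score HUD's fadeout once.
; Escape or P pauses the game and BP_AudioManager's music, shows the pause HUD and plays a tone, with no unpause logic here.
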(event `self.ReceiveBeginPlay`
  (`self.EnableInput` (`GameplayStatics.GetPlayerController` 0))
  ; Reference score widget and initialize score
  (bind _returnvalue (`|CreateWidget` "/Game/Blueprints/Pawn/Widgets/ScoreHUD.ScoreHUD_C"))
  (bind _output_get (set `self.Score HUD` _returnvalue))
  (`UserWidget.AddToViewport` _output_get 0)
  ; Reference pause widget
  (bind _returnvalue_2 (`|CreateWidget` "/Game/Blueprints/Pawn/Widgets/PauseHUD.PauseHUD_C"))
  (set `self.Pause HUD` _returnvalue_2)
  (set `self.Current Score` 0))

(event `self.ReceiveTick`
  (params (DeltaSeconds :type "Float (single-precision)"))
  (bind _score_hud (`self.Score HUD`))
  ; Constantly check for when game is over
  (if (`self.Is Game Over?`)
    (`/Engine/EditorBlueprintResources/StandardMacros.DoOnce` false
      (:`Completed`
        (set `Widget.Visibility` "Visible" (`/Game/Blueprints/Pawn/Widgets/ScoreHUD.FadeoutCover` _score_hud))
        (`/Game/Blueprints/Pawn/Widgets/ScoreHUD.Play Fadeout` _score_hud)))))

(event `Key|Escape`
  (params (Key :type "Key Structure"))
  (:`Pressed`
    ; Pause game
    (set `PlayerController.bShowMouseCursor` false (`GameplayStatics.GetPlayerController` 0) :!label _label)
    (`GameplayStatics.SetGamePaused` true)
    ; Pause music
    (bind _returnvalue (`GameplayStatics.GetActorOfClass` "/Game/Blueprints/Pawn/BP_AudioManager.BP_AudioManager_C"))
    (bind _output_get (set `self.Audio Manager REF` _returnvalue))
    (`AudioComponent.SetPaused` (`/Game/Blueprints/Pawn/BP_AudioManager.Music REF` _output_get) true)
    ; Show pause menu
    (`UserWidget.AddToViewport` (`self.Pause HUD`) 0)
    (set `self.Is Game Paused?` true)
    (`GameplayStatics.PlaySound2D` "/Game/Assets/Sounds/pause_tone_Cue.pause_tone_Cue" 1.0 1.0 0.0 null null)))

(event `Key|P`
  (params (Key :type "Key Structure"))
  (:`Pressed`
    (goto _label)))

(fn `UserConstructionScript`)